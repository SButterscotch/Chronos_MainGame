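; Gate door actor that toggles on a floor-trigger overlap and leads to a teleport into the main level.
; A FlipFlop alternates playing and reversing a timeline, whose update sets the door mesh's relative location through a vertical lerp with Alpha fixed at zero.
; That update also enables query collision on the teleport box, whose overlap opens Lvl_Main.
; A separate ShowLever event makes the lever visible.
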(event `self.Box.OnComponentBeginOverlap`
  (params (OverlappedComponent :type "PrimitiveComponent Object Reference") (OtherActor :type "Actor Object Reference") (OtherComp :type "PrimitiveComponent Object Reference") (OtherBodyIndex :type Integer) (bFromSweep :type Boolean) (SweepResult :type "HitResult Structure (by ref)"))
  (`KismetSystemLibrary.PrintText` "Passed Floor Button")
  (`self.Toggle Door`))

(event `Show Lever`
  (`SceneComponent.SetVisibility` (`self.Lever`) true false))

(event `Toggle Door`
  (`/Engine/EditorBlueprintResources/StandardMacros.FlipFlop`
    (:`A`
      (`Timeline|Door Open/Close` :!label _label
        (:`Update`
          (`SceneComponent.K2_SetRelativeLocation` (`self.DoorMesh`) (`KismetMathLibrary.VLerp` (0.0 0.0 -200.0)) false false)
          (`self.Spawn Teleport`))))
    (:`B`
      (goto _label :!via `Reverse`))))

(event `Spawn Teleport`
  (`PrimitiveComponent.SetCollisionEnabled` (`self.TeleportBoex`) "QueryOnly"))

(event `self.TeleportBoex.OnComponentBeginOverlap`
  (params (OverlappedComponent :type "PrimitiveComponent Object Reference") (OtherActor :type "Actor Object Reference") (OtherComp :type "PrimitiveComponent Object Reference") (OtherBodyIndex :type Integer) (bFromSweep :type Boolean) (SweepResult :type "HitResult Structure (by ref)"))
  (`KismetSystemLibrary.PrintText` "Pass Teleport Box")
  (`GameplayStatics.OpenLevelBySoftObjectPtr` "/Game/Maps/Lvl_Main.Lvl_Main"))

(fn `UserConstructionScript`)