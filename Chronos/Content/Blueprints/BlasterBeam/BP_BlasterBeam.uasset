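; BP_BlasterBeam is a blaster beam projectile actor that reacts when its Box component hits something.
; The hit event passes the actor and result to HandleOnIt, which spawns a Niagara burst at the impact point, oriented along the hit normal.
; If the hit actor is TargetPawn the game quits outright; otherwise the beam destroys itself.
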(event `self.ReceiveBeginPlay`)

(event `self.Box.OnComponentHit`
  (params (HitComponent :type "PrimitiveComponent Object Reference") (OtherActor :type "Actor Object Reference") (OtherComp :type "PrimitiveComponent Object Reference") (NormalImpulse :type "Vector Structure") (Hit :type "HitResult Structure (by ref)"))
  (`self.HandleOnIt` OtherActor Hit))

(fn `HandleOnIt`
  (params (HitActor :type "Object Object Reference") (HitResult :type "HitResult Structure (by ref)"))
  (bind (_bblockinghit _binitialoverlap _time _distance _location _impactpoint _normal) (`GameplayStatics.BreakHitResult` HitResult))
  (`NiagaraFunctionLibrary.SpawnSystemAtLocation` "/Game/Assets/FX/NS_BeamBurst.NS_BeamBurst" _impactpoint (`KismetMathLibrary.MakeRotFromX` _normal))
  (if (== (`local.HitActor`) (`self.TargetPawn`))
    (`KismetSystemLibrary.QuitGame` null "Quit")
    (else
      (`self.K2_DestroyActor`))))

(fn `UserConstructionScript`)