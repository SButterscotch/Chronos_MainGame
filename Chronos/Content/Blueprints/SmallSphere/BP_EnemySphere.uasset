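; Small sphere enemy that homes in on the top-down player character and damages it on contact.
; On BeginPlay it scales in by timeline and stores the first BP_TopDownCharacter found as its target.
; Each tick it smoothly turns toward the target, moving forward only while facing it within a threshold.
; Overlap damages the player, then scales the sphere out and destroys it; the timed fade-out is disconnected.
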(event `self.ReceiveBeginPlay`
  (`self.FadeIn`)
  (`self.StoreTargetPawn`))

(event `FadeOut`
  ;[0.15 0.0159 0.0202 0.5] fade Out
  (bind (_direction _scale) (`Timeline|FadeOutTimeline`)
    (:`Update`
      (`SceneComponent.SetWorldScale3D` (`self.SphereMesh`) (`KismetMathLibrary.Conv_DoubleToVector` (* _scale (`self.SphereSize`)))))
    (:`Finished`
      (`self.K2_DestroyActor`))))

(event `FadeIn`
  ;[0.15 0 0.01576 0.5] Fade IN
  (bind (_direction _scale) (`Timeline|FadeInTimeline`)
    (:`Update`
      (`SceneComponent.SetWorldScale3D` (`self.SphereMesh`) (* _scale (`self.SphereSize`))))))

(event `self.ReceiveTick`
  (params (DeltaSeconds :type "Float (single-precision)"))
  (`self.RotateToPlayer`)
  (bind _islooking (`self.IsLooking`))
  (if _islooking
    (`self.MoveToPawn`)))

(event `self.SphereVolume.OnComponentBeginOverlap`
  (params (OverlappedComponent :type "PrimitiveComponent Object Reference") (OtherActor :type "Actor Object Reference") (OtherComp :type "PrimitiveComponent Object Reference") (OtherBodyIndex :type Integer) (bFromSweep :type Boolean) (SweepResult :type "HitResult Structure (by ref)"))
  (bind _asbp_top_down_character (cast `/Game/Blueprints/Player/BP_TopDownCharacter` OtherActor))
  (`/Game/Blueprints/Player/BP_TopDownCharacter.PlayerTakeDamage` _asbp_top_down_character)
  (`self.FadeOut`))

(fn `IsLooking`
  (returns (IsLooking :type Boolean))
  (if (== (`self.K2_GetActorRotation`) (`KismetMathLibrary.FindLookAtRotation` (`self.K2_GetActorLocation`) (`self.K2_GetActorLocation` (`self.TargetPawn`))) :`ErrorTolerance` (`self.SpotThreshold`))
    (return true)))

(fn `MovetoPawn`
  (`self.K2_AddActorWorldOffset` (* (`self.GetActorForwardVector`) (* (`self.Speed`) (* (`GameplayStatics.GetWorldDeltaSeconds`) 100.0)))))

(fn `RotateToPlayer`
  (`|ExecutionSequence`
    (:`then_0`
      ; Turn to Pawn (Player)
      (`self.TargetPawn`
        (:`then`
          (`self.K2_SetActorRotation` (`KismetMathLibrary.RInterpTo` (`self.K2_GetActorRotation`) (`KismetMathLibrary.FindLookAtRotation` (`self.K2_GetActorLocation`) (`self.K2_GetActorLocation` (`self.TargetPawn`))) (`GameplayStatics.GetWorldDeltaSeconds`) (`self.RotationInterpSpeed`))))
        (:`else`)))))

(fn `SetRotation`
  (set `self.Rotator` (* (`KismetMathLibrary.RandomRotator` false) (`self.RandomRotationFactor`))))

(fn `StoreTargetPawn`
  (bind _outactors (`GameplayStatics.GetAllActorsOfClass` "/Game/Blueprints/Player/BP_TopDownCharacter.BP_TopDownCharacter_C"))
  (if (`KismetArrayLibrary.Array_IsValidIndex` _outactors)
    (set `self.TargetPawn` (`|GetArrayItem` _outactors))))

(fn `UserConstructionScript`)