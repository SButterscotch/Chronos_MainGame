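; BP_EnemySpawner is an actor that spawns BP_EnemySphere enemies at random points within SpawnRadius around itself.
; BeginPlay records the player's level and starts a looping timer on the initial SpawnRate interval.
; Tick lowers SpawnRate toward zero while the player's level exceeds that starting level, which is never updated.
; The timer is never reset, so these reductions do not change the actual spawn interval.
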(event `self.ReceiveTick`
  (params (DeltaSeconds :type "Float (single-precision)"))
  (bind _asbp_top_down_character (cast `/Game/Blueprints/Player/BP_TopDownCharacter` (`GameplayStatics.GetPlayerCharacter` 0)))
  (if (> (`/Game/Blueprints/Player/BP_TopDownCharacter.PlayerLevel` _asbp_top_down_character) (`self.prevlevel`))
    (if (!= (`self.SpawnRate`) 0.0)
      (set `self.SpawnRate` (- (`self.SpawnRate`) 2.0)))))

(event `self.ReceiveBeginPlay`
  (`|ExecutionSequence`
    (:`then_0`
      (bind _asbp_top_down_character (cast `/Game/Blueprints/Player/BP_TopDownCharacter` (`GameplayStatics.GetPlayerCharacter` 0)))
      (set `self.prevlevel` (`/Game/Blueprints/Player/BP_TopDownCharacter.PlayerLevel` _asbp_top_down_character))
      (set `self.SpawnRate` 10.0))
    (:`then_1`
      (`KismetSystemLibrary.K2_SetTimerDelegate` (delegate `SpawnHead`) (`self.SpawnRate`) true))))

(event `SpawnHead`
  (`|SpawnActorFromClass` "/Game/Blueprints/SmallSphere/BP_EnemySphere.BP_EnemySphere_C" (`KismetMathLibrary.MakeTransform` (`self.GetRandomPointinSphere`) (`KismetMathLibrary.RandomRotator` false)) "Undefined" "MultiplyWithRoot" null null))

(fn `GetRandomPointinSphere`
  (returns (RandomPoint :type "Vector Structure"))
  (return (+ (`self.K2_GetActorLocation`) (* (`KismetMathLibrary.GetForwardVector` (`KismetMathLibrary.RandomRotator` false)) (`KismetMathLibrary.RandomFloatInRange` 0.0 (`self.SpawnRadius`))))))

(fn `UserConstructionScript`)